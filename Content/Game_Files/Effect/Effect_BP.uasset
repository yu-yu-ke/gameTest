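; Impact effect actor that plays bullet-hit feedback on BeginPlay when its stored hit result is a blocking hit.
; The physical material's surface type selects particle and sound from EffectInfo for stone, metal, wood or skin, with body-part surfaces sharing skin effects.
; A crater decal, aligned to the hit normal with random roll, attaches to the hit component and bone.
; The actor's lifespan matches the decal's.
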(event EventBeginPlay
  (bind _命中结果 (Variables|Default|Get命中结果))
  (bind _effect_info (Variables|Default|GetEffect_Info))
  (bind _命中结果_2 (Variables|Default|Get命中结果))
  (bind _effect_info_2 (Variables|Default|GetEffect_Info))
  (bind _命中结果_3 (Variables|Default|Get命中结果))
  (bind _命中结果_4 (Variables|Default|Get命中结果))
  (bind _effect_info_3 (Variables|Default|GetEffect_Info))
  (bind (_击中石头的特效粒子 _击中皮肤的特效粒子 _击中金属的特效粒子 _击中木头的特效粒子) (Utilities|Struct|BreakEffect_Info _effect_info))
  (bind (_击中石头的音效 _击中皮肤的音效 _击中金属的音效 _击中木头的音效) (Utilities|Struct|BreakEffect_Info _effect_info_2))
  (bind (_击中后产生的弹坑材质 _弹坑材质所存在的时间 _弹坑的大小) (Utilities|Struct|BreakEffect_Info _effect_info_3))
  (bind (_bblockinghit _binitialoverlap _time _distance _location _impactpoint _normal _impactnormal _physmat _hitactor _hitcomponent _hitbonename) (Collision|BreakHitResult _命中结果))
  (bind (_bblockinghit_2 _binitialoverlap_2 _time_2 _distance_2 _location_2 _impactpoint_2 _normal_2) (Collision|BreakHitResult _命中结果_4))
  (bind (_bblockinghit_3 _binitialoverlap_3 _time_3 _distance_3 _location_3 _impactpoint_3 _normal_3 _impactnormal_2 _physmat_2) (Collision|BreakHitResult _命中结果_2))
  (bind (_bblockinghit_4 _binitialoverlap_4 _time_4 _distance_4 _location_4 _impactpoint_4 _normal_4 _impactnormal_3 _physmat_3) (Collision|BreakHitResult _命中结果_3))
  (bind _returnvalue (Math|Conversions|RotationFromXVector _normal_2))
  (bind (_roll _pitch _yaw) (Math|Rotator|BreakRotator _returnvalue))
  (Utilities|FlowControl|Sequence
    (:then_0
      (if _bblockinghit_3
        (Effects|SpawnEmitteratLocation (Utilities|Select :Index (Variables|/Script/PhysicsCore.PhysicalMaterial|GetSurfaceType _physmat_2) :SurfaceType_Default _击中石头的特效粒子 :SurfaceType1 _击中石头的特效粒子 :SurfaceType2 _击中金属的特效粒子 :SurfaceType3 _击中木头的特效粒子 :SurfaceType4 _击中皮肤的特效粒子 :SurfaceType5 _击中皮肤的特效粒子 :SurfaceType6 _击中皮肤的特效粒子 :SurfaceType7 _击中皮肤的特效粒子 :SurfaceType8 _击中皮肤的特效粒子) _impactpoint_3)))
    (:then_1
      (if _bblockinghit_4
        (Audio|SpawnSoundatLocation (Utilities|Select :Index (Variables|/Script/PhysicsCore.PhysicalMaterial|GetSurfaceType _physmat_3) :SurfaceType_Default _击中石头的音效 :SurfaceType1 _击中石头的音效 :SurfaceType2 _击中金属的音效 :SurfaceType3 _击中木头的音效 :SurfaceType4 _击中皮肤的音效 :SurfaceType5 _击中皮肤的音效 :SurfaceType6 _击中皮肤的音效 :SurfaceType7 _击中皮肤的音效 :SurfaceType8 _击中皮肤的音效) _impactpoint_4 "0, 0, 0" 1.0 1.0 0.0 0 0)))
    (:then_2
      (if _bblockinghit_2
        (Variables|Default|SetDetal_Rotation (Math|Rotator|MakeRotator (Math|Random|RandomFloatinRange -1.8e+02 1.8e+02) _pitch _yaw))))
    (:then_3
      (if _bblockinghit
        (Class|GameplayStatics|SpawnDecalAttached _击中后产生的弹坑材质 (Math|Vector|MakeVector _弹坑的大小 _弹坑的大小 _弹坑的大小) _hitcomponent _hitbonename _impactpoint (Variables|Default|GetDetal_Rotation) "KeepWorldPosition" _弹坑材质所存在的时间)
        (Actor|SetLifeSpan _弹坑材质所存在的时间)))))

(fn ConstructionScript)
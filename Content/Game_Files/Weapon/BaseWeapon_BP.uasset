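; Base weapon Blueprint that acts as a world pickup for Ke_Charactor_BP and carries its stats and assets in a WeaponInfo struct.
; Sphere overlap toggles the prompt widget and CanPickUp, registers or clears the character's OverlapWeapon, and fills PickUp_UI with name and icon.
; The construction script stamps the actor's own class into WeaponInfo.
; CloseComponentEvent disables sphere collision and hides the prompt, while the picked-up event 枪被捡起 only performs checks.
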(event OnComponentBeginOverlap(Sphere)
  (params (OverlappedComponent :type Primitive%20Component%20Object%20Reference) (OtherActor :type Actor%20Object%20Reference) (OtherComp :type Primitive%20Component%20Object%20Reference) (OtherBodyIndex :type Integer) (bFromSweep :type Boolean) (SweepResult :type Hit%20Result%20Structure%20%28by%20ref%29))
  (bind _widget (Variables|Default|GetWidget))
  (bind _weapon_info (Variables|Default|GetWeapon_info))
  (bind (_图标 _武器名称) (Utilities|Struct|Breakweapon_Info _weapon_info))
  (bind _returnvalue (UserInterface|GetUserWidgetObject _widget))
  (bind _aspick_up_ui (Utilities|Casting|CastToPickUp_UI _returnvalue))
  (bind _aske_charactor_bp (Utilities|Casting|CastToKe_Charactor_BP OtherActor))
  (Variables|Default|SetAs%20Ke%20Charactor%20BP _aske_charactor_bp)
  (Rendering|SetVisibility (Variables|Default|GetWidget) true false)
  (Variables|Default|SetCanPickUp? true)
  ;[1 1 1] 设置重叠时的武器
  (Variables|/Game/Game_Files/Charactor/Ke_Charactor_BP.Ke_Charactor_BP_C|SetOverlapWeapon (Variables|Default|GetAs%20Ke%20Charactor%20BP) self)
  (Variables|/Game/Game_Files/Game_UI/PickUp_UI.PickUp_UI_C|Set武器名称_name _aspick_up_ui (Utilities|Text|ToText(String) _武器名称))
  (Variables|/Game/Game_Files/Game_UI/PickUp_UI.PickUp_UI_C|Set武器图标_image _aspick_up_ui _图标))

(event OnComponentEndOverlap(Sphere)
  (params (OverlappedComponent :type Primitive%20Component%20Object%20Reference) (OtherActor :type Actor%20Object%20Reference) (OtherComp :type Primitive%20Component%20Object%20Reference) (OtherBodyIndex :type Integer))
  (bind _aske_charactor_bp (Utilities|Casting|CastToKe_Charactor_BP OtherActor))
  (Variables|Default|SetAs%20Ke%20Charactor%20BP _aske_charactor_bp)
  (Rendering|SetVisibility (Variables|Default|GetWidget) false false)
  (Variables|Default|SetCanPickUp? false)
  ;[1 1 1] 取消重叠时的武器
  (Variables|/Game/Game_Files/Charactor/Ke_Charactor_BP.Ke_Charactor_BP_C|SetOverlapWeapon (Variables|Default|GetAs%20Ke%20Charactor%20BP) 0))

(event Custom|CloseComponentEvent
  ;[1 1 1] 清除组件的功能
  (Collision|SetCollisionEnabled (Variables|Default|GetSphere) "NoCollision")
  (Rendering|SetVisibility (Variables|Default|GetWidget) false false))

(event Custom|枪被捡起
  (Utilities|IsValid (Variables|Default|GetAs%20Ke%20Charactor%20BP)
    (:Is%20Valid
      (if (Variables|Default|GetCanPickUp?)
        _))))

(fn ConstructionScript
  (Variables|Default|SetWeapon_info (Utilities|Struct|Makeweapon_Info (.weapontype (Variables|Default|GetWeapon_info)) (Utilities|GetClass self) (.图标 (Variables|Default|GetWeapon_info)) (.武器名称 (Variables|Default|GetWeapon_info)) (.射击速度 (Variables|Default|GetWeapon_info)) (.开火声音 (Variables|Default|GetWeapon_info)) (.当前装弹量 (Variables|Default|GetWeapon_info)) (.弹夹载弹量 (Variables|Default|GetWeapon_info)) (.maxammo (Variables|Default|GetWeapon_info)) (.武器伤害值 (Variables|Default|GetWeapon_info)) (.weaponholdsocket (Variables|Default|GetWeapon_info)) (.weaponequipsocket (Variables|Default|GetWeapon_info)) (.unequipsound (Variables|Default|GetWeapon_info)) (.equipsound (Variables|Default|GetWeapon_info)) (.射击距离 (Variables|Default|GetWeapon_info)) (.射击蒙太奇 (Variables|Default|GetWeapon_info)) (.武器空弹声音 (Variables|Default|GetWeapon_info)) (.武器重装弹药蒙太奇 (Variables|Default|GetWeapon_info)) (.弹夹类型 (Variables|Default|GetWeapon_info)))))
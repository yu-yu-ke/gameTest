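; Zombie enemy character that wanders random navmesh points until damaged, then chases and attacks the player.
; An AI MoveTo and montage loop drives attacks; collision overlap damages the player while the attack window is open.
; Bullet damage scales by physical material, radial damage by impact distance, and grenade damage applies directly, all updating a health-bar widget.
; Death hides the bar, then restores health and saved transform after a delay; the ragdoll function is never called here.
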(event OnComponentBeginOverlap(攻击碰撞体)
  (params (OverlappedComponent :type Primitive%20Component%20Object%20Reference) (OtherActor :type Actor%20Object%20Reference) (OtherComp :type Primitive%20Component%20Object%20Reference) (OtherBodyIndex :type Integer) (bFromSweep :type Boolean) (SweepResult :type Hit%20Result%20Structure%20%28by%20ref%29))
  ;[1 1 1] 攻击碰撞体
  (if (Variables|Default|GetSphereAttackValid?)
    (bind _aske_charactor_bp (Utilities|Casting|CastToKe_Charactor_BP OtherActor))
    (bind _output_get (Variables|Default|SetPlayer _aske_charactor_bp))
    (Class|DamageInterface|TransimitDamage(Message) _output_get (Variables|Default|Get攻击力))))

(event OnComponentEndOverlap(攻击碰撞体)
  (params (OverlappedComponent :type Primitive%20Component%20Object%20Reference) (OtherActor :type Actor%20Object%20Reference) (OtherComp :type Primitive%20Component%20Object%20Reference) (OtherBodyIndex :type Integer))
  ;[1 1 1] 攻击碰撞体
  (Variables|Default|SetPlayer 0))

(event Custom|追捕玩家
  ;[1 1 1] 追捕与攻击玩家
  (if (Variables|Default|GetAttackPlayer?)
    (if (not (Variables|Default|GetIsDeath?))
      (Variables|/Script/Engine.CharacterMovementComponent|SetMaxWalkSpeed (Variables|Character|GetCharacterMovement) 4.5e+02)
      (AI|AIMoveTo self "0, 0, 0" (Game|GetPlayerCharacter 0) 5.0 false
        (:OnSuccess
          (CallFunction|AI攻击玩家))
        (:OnFail
          (CallFunction|追捕玩家))))))

(event Custom|怪物移动
  ;[1 1 1] 怪物移动
  (if (not (Variables|Default|GetIsDeath?))
    (AI|AIMoveTo self (.RandomLocation (Class|NavigationSystemV1|GetRandomPointinNavigableRadius (Transformation|GetActorLocation) 1e+03 0 "/Script/AIModule.NavFilter_AIControllerDefault")) 0 5.0 false
      (:OnSuccess
        (Utilities|FlowControl|Delay (Math|Random|RandomFloatinRange 2.0 5.0))
        (CallFunction|怪物移动)))))

(event Custom|AI攻击玩家
  ;[1 1 1] 追捕与攻击玩家
  (if (Variables|Default|GetAttackPlayer?)
    (if (Variables|Default|GetPlayer%20Dead?)
      (Variables|/Script/Engine.CharacterMovementComponent|SetMaxWalkSpeed (Variables|Character|GetCharacterMovement) 1.8e+02)
      (CallFunction|怪物移动)
      (else
        (bind _returnvalue (Animation|PlayAnimMontage "/Game/Game_Files/Monster/Zoombie/Animation/Attack_Montage.Attack_Montage" 1.0 "None"))
        (Utilities|FlowControl|Delay _returnvalue)
        (CallFunction|追捕玩家)))))

(event Custom|开始攻击玩家
  ;[1 1 1] 攻击状态
  (Variables|Default|SetSphereAttackValid? true))

(event Custom|结束攻击玩家
  ;[1 1 1] 攻击状态
  (Variables|Default|SetSphereAttackValid? false))

(event EventGrenadeDamage
  (params (value :type Float%20%28single-precision%29) (explosion :type BP%20Explosion%20Object%20Reference))
  ;[1 1 1] 手榴弹爆炸伤害
  (if (not (Variables|Default|GetIsDeath?))
    (bind _死亡_ (CallFunction|更新生命值 value))
    (CallFunction|UI更新函数)
    (if _死亡_
      (Utilities|怪物重新复活)
      (else
        (CallFunction|追捕玩家)
        (Variables|Default|SetAttackPlayer? true)))))

(event EventBeginPlay
  (bind _returnvalue (Game|Player|GetPlayerPawn 0))
  (bind _self self)
  (bind _returnvalue_2 (Actor|GetComponentbyClass _returnvalue "/Game/Game_Files/WeaponComponent/WeaponComponent.WeaponComponent_C"))
  ;[1 1 1] 怪物移动
  (CallFunction|怪物移动)
  (Variables|Default|SetCurrHealth (Variables|Default|GetMaxHealth))
  (CallFunction|UI更新函数)
  (Utilities|IsValid _returnvalue_2
    (:Is%20Valid
      (Variables|组件|SetWeaponComponent_Ref _returnvalue_2)
      (Variables|Default|SetAIControllerClass _self "/Game/Game_Files/Target/AI_Controller.AI_Controller_C")
      (Variables|Default|Settransform (Transformation|GetActorTransform _self)))))

(event EventTick
  (params (DeltaSeconds :type Float%20%28single-precision%29))
  (bind _player (Variables|Default|GetPlayer))
  ;[1 1 1] 持续攻击player
  (Utilities|IsValid _player
    (:Is%20Valid
      (Variables|Default|SetPlayer%20Dead? (Variables|/Game/Game_Files/Charactor/Ke_Charactor_BP.Ke_Charactor_BP_C|GetPlayerDead? _player)))))

(event EventTransimitRadiusDamage
  (params (命中结果 :type Hit%20Result%20Structure) (子弹信息 :type Ammo%20Info%20Structure))
  ;[1 1 1] new 怪物收到伤害
  (if (not (Variables|Default|GetIsDeath?))
    (bind _输出爆炸伤害 (CallFunction|计算爆炸性伤害 命中结果 子弹信息))
    (bind _死亡_ (CallFunction|更新生命值 _输出爆炸伤害))
    (CallFunction|UI更新函数)
    (if _死亡_
      (Utilities|怪物重新复活)
      (else
        (CallFunction|追捕玩家)
        (Variables|Default|SetAttackPlayer? true)))))

(event EventTransimitDamage
  (params (命中结果 :type Hit%20Result%20Structure) (伤害值 :type Float%20%28single-precision%29))
  ;[1 1 1] new 怪物收到伤害
  (if (not (Variables|Default|GetIsDeath?))
    (bind _最后接收到的伤害 (CallFunction|计算所受伤害 命中结果 伤害值))
    (bind _死亡_ (CallFunction|更新生命值 _最后接收到的伤害))
    (CallFunction|UI更新函数)
    (if _死亡_
      (Utilities|怪物重新复活)
      (else
        (CallFunction|追捕玩家)
        (Variables|Default|SetAttackPlayer? true)))))

(fn ConstructionScript)

(fn UI更新函数
  (bind _aszoombie_ui (Utilities|Casting|CastToZoombie_UI (UserInterface|GetUserWidgetObject (Variables|Default|GetWidget))))
  (bind _output_get (Variables|Default|Set怪物UI _aszoombie_ui))
  (Progress|SetPercent (Variables|/Game/Game_Files/Monster/Zoombie/Blueprints/Zoombie_UI.Zoombie_UI_C|Get怪物生命值 _output_get) (/ (Variables|Default|GetCurrHealth) (Variables|Default|GetMaxHealth))))

(fn 计算所受伤害
  (params (命中结果 :type Hit%20Result%20Structure) (Damage :type Float%20%28single-precision%29))
  (return (* (Variables|/Script/PhysicsCore.PhysicalMaterial|GetDestructibleDamageThresholdScale (.PhysMat (Collision|BreakHitResult 命中结果))) Damage)))

(fn 更新生命值
  (params (伤害值 :type Float%20%28single-precision%29))
  (if (<= (- (Variables|Default|GetCurrHealth) 伤害值) 0.0)
    (Variables|Default|SetIsDeath? true)
    (Variables|Default|SetCurrHealth 0.0)
    (else
      (Variables|Default|SetCurrHealth (- (Variables|Default|GetCurrHealth) 伤害值))))
  (return (Variables|Default|GetIsDeath?)))

(fn Target死亡
  (params (命中结果 :type Hit%20Result%20Structure))
  (bind (_bblockinghit _binitialoverlap _time _distance _location _impactpoint _normal _impactnormal _physmat _hitactor _hitcomponent _hitbonename) (Collision|BreakHitResult 命中结果))
  (bind _mesh (Variables|Character|GetMesh))
  (bind _weaponcomponent_ref (Variables|组件|GetWeaponComponent_Ref))
  (bind _currentweapon (Variables|/Game/Game_Files/WeaponComponent/WeaponComponent.WeaponComponent_C|GetCurrentWeapon _weaponcomponent_ref))
  (bind _weapon_info (Variables|/Game/Game_Files/Item/Weapon_Child/Weapon_BP_Child.Weapon_BP_Child_C|GetWeapon_Info _currentweapon))
  (bind (_射击距离 _武器伤害) (Utilities|Struct|BreakWeapon_Info _weapon_info))
  (Utilities|FlowControl|Sequence
    (:then_0
      (Collision|SetCollisionEnabled _mesh "QueryAndPhysics")
      (Physics|SetSimulatePhysics _mesh true))
    (:then_2
      (Physics|AddImpulseatLocation (Variables|Character|GetMesh) (* (Math|Vector|Normalize (- _impactpoint (Transformation|GetActorLocation _currentweapon)) _射击距离) (Math|Float|Power _武器伤害 2.0)) _impactpoint _hitbonename))))

(fn 计算爆炸性伤害
  (params (命中结果 :type Hit%20Result%20Structure) (Ammo_Info :type Ammo%20Info%20Structure))
  (bind (_径向爆炸伤害值 _爆炸半径) (Utilities|Struct|BreakAmmo_Info Ammo_Info))
  (bind (_bblockinghit _binitialoverlap _time _distance _location _impactpoint) (Collision|BreakHitResult 命中结果))
  (if _bblockinghit
    (bind _output_get (LocalVariables|Set爆炸物落点 _impactpoint))
    (if (< (Math|Vector|VectorLength (- _output_get (Transformation|GetActorLocation self))) _爆炸半径)
      (return (* (/ (Math|Vector|VectorLength (- _output_get (Transformation|GetActorLocation self))) _爆炸半径) _径向爆炸伤害值)))))
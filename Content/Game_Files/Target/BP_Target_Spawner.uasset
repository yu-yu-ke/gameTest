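; BP_Target_Spawner keeps spawning BP_Target actors at random points inside its SpawnerArea box.
; A looping one-second timer spawns a target only while the level holds ten or fewer, counted with GetAllActorsOfClass.
; Each target is rotated toward the player camera with a yaw offset, and its position is adjusted for collisions.
; The construction script sizes the box from the BoxExtent variable.
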(event Custom|SpawnerTarget
  (bind _spawner_area (Variables|Default|GetSpawner_Area))
  (bind _outactors (Actor|GetAllActorsOfClass "/Game/Game_Files/Target/BP_Target.BP_Target_C"))
  (if (<= (Utilities|Array|Length _outactors) 10)
    (bind _output_get (Variables|Default|SetSpawnLocation (Math|Random|RandomPointinBoundingBox (Transformation|GetWorldLocation _spawner_area) (Components|Box|GetScaledBoxExtent _spawner_area))))
    (Game|SpawnActorfromClass "/Game/Game_Files/Target/BP_Target.BP_Target_C" (Math|Transform|MakeTransform _output_get (Math|Rotator|MakeRotator (.roll (Math|Rotator|FindLookatRotation _output_get (Transformation|GetWorldLocation (Variables|/Script/Engine.PlayerCameraManager|GetTransformComponent (Game|GetPlayerCameraManager 0))))) (.pitch (Math|Rotator|FindLookatRotation _output_get (Transformation|GetWorldLocation (Variables|/Script/Engine.PlayerCameraManager|GetTransformComponent (Game|GetPlayerCameraManager 0))))) (- (.yaw (Math|Rotator|FindLookatRotation _output_get (Transformation|GetWorldLocation (Variables|/Script/Engine.PlayerCameraManager|GetTransformComponent (Game|GetPlayerCameraManager 0))))) 9e+01)) "1,1,1") "AdjustIfPossibleButAlwaysSpawn" 0 0)))

(event EventBeginPlay
  (Utilities|Time|SetTimerbyEvent (delegate Custom|SpawnerTarget) 1.0 true))

(fn ConstructionScript
  (Components|Box|SetBoxExtent (Variables|Default|GetSpawner_Area) (Variables|Default|GetBox%20Extent) true))
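; Shooting target actor that gets a random size and behavior on construction: sliding horizontally, moving vertically or pulsing in scale, driven by a timeline at random speed.
; Damage events subtract health, scaling hits by physical material and blasts by distance/radius, so blast damage rises toward the edge.
; On death it expires shortly after; hit and radius kills also enable physics and play a collapse sound, while grenade kills skip both.
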(event EventGrenadeDamage
  (params (value :type Float%20%28single-precision%29) (explosion :type BP%20Explosion%20Object%20Reference))
  (if (not (Variables|Default|Get是否死亡？))
    (bind _死亡_ (CallFunction|更新生命值 value))
    (if _死亡_
      (Actor|SetLifeSpan 0.2))))

(event EventBeginPlay
  (bind _returnvalue (Math|Random|RandomFloatinRange 1e+02 2.5e+02))
  (bind _returnvalue_2 (Game|Player|GetPlayerPawn 0))
  (bind _staticmesh (Variables|Default|GetStaticMesh))
  (bind _actorscale (Variables|Default|GetActorScale))
  (bind _returnvalue_3 (Actor|GetComponentbyClass _returnvalue_2 "/Game/Game_Files/WeaponComponent/WeaponComponent.WeaponComponent_C"))
  (bind _returnvalue_4 (* _actorscale 1.5))
  (switch Utilities|FlowControl|Switch|SwitchonE_targetBehavior (Variables|Default|GetTargetBehavior)
    (:NewEnumerator1
      (Variables|Default|SetDestinationLocation (Math|Vector|MakeVector _returnvalue 0.0 0.0)))
    (:NewEnumerator2
      (Variables|Default|SetDestinationLocation (Math|Vector|MakeVector 0.0 0.0 _returnvalue)))
    (:NewEnumerator3
      _))
  (Components|Timeline|SetPlayRate (Variables|Default|Get时间轴_0) (/ 1.0 (Math|Random|RandomFloatinRange 1.5 3.0)))
  (bind _alpha (Timeline|时间轴_0 PlayFromStart)
    (:Update
      (switch Utilities|FlowControl|Switch|SwitchonE_targetBehavior (Variables|Default|GetTargetBehavior)
        (:NewEnumerator1
          (Transformation|SetRelativeLocation _staticmesh (Math|Vector|Lerp(Vector) "0, 0, 0" (Variables|Default|GetDestinationLocation) _alpha) false false :!label _label)
          (Utilities|IsValid _returnvalue_3
            (:Is%20Valid
              (Variables|Default|SetWeaponComponentRef _returnvalue_3))))
        (:NewEnumerator2
          (goto _label))
        (:NewEnumerator3
          (Transformation|SetWorldScale3D _staticmesh (Math|Vector|Lerp(Vector) (Math|Vector|MakeVector _actorscale _actorscale _actorscale) (Math|Vector|MakeVector _returnvalue_4 _returnvalue_4 _returnvalue_4) _alpha)))))))

(event EventTransimitDamage
  (params (命中结果 :type Hit%20Result%20Structure) (伤害值 :type Float%20%28single-precision%29))
  (if (not (Variables|Default|Get是否死亡？))
    (bind _最后接收到的伤害 (CallFunction|计算所受伤害 命中结果 伤害值))
    (bind _死亡_ (CallFunction|更新生命值 _最后接收到的伤害))
    (if _死亡_
      (CallFunction|Target死亡 命中结果)
      (Actor|SetLifeSpan 0.5))))

(event EventTransimitRadiusDamage
  (params (命中结果 :type Hit%20Result%20Structure) (子弹信息 :type Ammo%20Info%20Structure))
  (if (not (Variables|Default|Get是否死亡？))
    (bind _输出爆炸伤害 (CallFunction|计算爆炸性伤害 命中结果 子弹信息))
    (bind _死亡_ (CallFunction|更新生命值 _输出爆炸伤害))
    (if _死亡_
      (CallFunction|Target死亡 命中结果)
      (Actor|SetLifeSpan 0.5))))

(fn ConstructionScript
  (bind _output_get (Variables|Default|SetActorScale (Math|Random|RandomFloatinRange 0.25 1.0)))
  (Transformation|SetWorldScale3D (Variables|Default|GetStaticMesh) (Math|Vector|MakeVector _output_get _output_get _output_get))
  (Variables|Default|SetTargetBehavior (Utilities|Enum|ByteToEnumE_targetBehavior (Math|Conversions|ToByte(Integer) (Math|Random|RandomIntegerinRange 1 3))))
  (Variables|Default|Set当前生命值 (Variables|Default|Get最大生命值)))

(fn 计算所受伤害
  (params (命中结果 :type Hit%20Result%20Structure) (Damage :type Float%20%28single-precision%29))
  (return (* (Variables|/Script/PhysicsCore.PhysicalMaterial|GetDestructibleDamageThresholdScale (.PhysMat (Collision|BreakHitResult 命中结果))) Damage)))

(fn 更新生命值
  (params (伤害值 :type Float%20%28single-precision%29))
  (if (<= (- (Variables|Default|Get当前生命值) 伤害值) 0.0)
    (Variables|Default|Set是否死亡？ true)
    (Variables|Default|Set当前生命值 0.0)
    (else
      (Variables|Default|Set当前生命值 (- (Variables|Default|Get当前生命值) 伤害值))))
  (return (Variables|Default|Get是否死亡？)))

(fn Target死亡
  (params (命中结果 :type Hit%20Result%20Structure))
  (bind _staticmesh (Variables|Default|GetStaticMesh))
  (Utilities|FlowControl|Sequence
    (:then_0
      (Collision|SetCollisionEnabled _staticmesh "QueryAndPhysics")
      (Physics|SetSimulatePhysics _staticmesh true))
    (:then_1
      (Audio|PlaySound2D "/Game/MobileStarterContent/Audio/Collapse01.Collapse01" 1.0 1.0 0.0 0 0))))

(fn 计算爆炸性伤害
  (params (命中结果 :type Hit%20Result%20Structure) (Ammo_Info :type Ammo%20Info%20Structure))
  (bind (_径向爆炸伤害值 _爆炸半径) (Utilities|Struct|BreakAmmo_Info Ammo_Info))
  (bind (_bblockinghit _binitialoverlap _time _distance _location _impactpoint) (Collision|BreakHitResult 命中结果))
  (if _bblockinghit
    (bind _output_get (LocalVariables|Set爆炸物落点 _impactpoint))
    (if (< (Math|Vector|VectorLength (- _output_get (Transformation|GetActorLocation self))) _爆炸半径)
      (return (* (/ (Math|Vector|VectorLength (- _output_get (Transformation|GetActorLocation self))) _爆炸半径) _径向爆炸伤害值)))))
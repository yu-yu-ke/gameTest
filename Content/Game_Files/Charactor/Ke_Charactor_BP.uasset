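; Player character Blueprint for a touch-controlled shooter, with a bottom HUD, virtual joysticks, movement, weapons and health.
; Weapon pickup, switching, dropping, firing and reloading delegate to WeaponComponent, while equip events handle montages, socket attachment and rotation mode.
; Timelines blend walk speed while armed and apply recoil pitch.
; A Tick-polled gate turns touch drags into camera rotation; damage plays hit reactions or disables input at zero health.
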(event EventBeginPlay
  (bind _returnvalue (Game|GetPlayerController 0))
  (Class|PlayerController|ActivateTouchInterface _returnvalue "/Game/Game_Files/Game_UI/DefaultVirtualJoysticks1.DefaultVirtualJoysticks1")
  (bind _returnvalue_2 (UserInterface|CreateWidget "/Game/Game_Files/Game_UI/Game_Bottom_UI.Game_Bottom_UI_C" _returnvalue))
  (bind _output_get (Variables|Default|SetNewVar_0 _returnvalue_2))
  (UserInterface|Viewport|AddtoViewport _output_get 0)
  (Variables|Default|SetCurrentHealth (Variables|Default|GetMaxHealth)))

(event Collision|EventActorBeginOverlap
  (params (OtherActor :type Actor%20Object%20Reference)))

(event EventTick
  (params (DeltaSeconds :type Float%20%28single-precision%29))
  (CallFunction|InputTouch))

(event Custom|jump%20end
  ;[1 1 1] 跳跃
  (Character|StopJumping))

(event Custom|jump%20start
  ;[1 1 1] 跳跃
  (Character|Jump))

(event Custom|丢弃武器
  ;[1 1 1] 丢弃武器
  (Default|丢弃武器 (Variables|Default|GetWeaponComponent)))

(event Custom|按压"fire"
  ;[1 1 1] 武器开火
  (Default|武器开火（由人物调用） (Variables|Default|GetWeaponComponent) true))

(event Custom|后座力Event
  (bind _returnvalue (Game|GetPlayerController 0))
  ;[1 1 1] 后座力
  (bind (_direction _新建轨道_0) (Timeline|时间轴_1 PlayFromStart)
    (:Update
      (switch Utilities|FlowControl|Switch|SwitchonETimelineDirection _direction
        (:Forward
          (Class|PlayerController|AddPitchInput _returnvalue (Math|Float|Lerp 0.0 -0.15 _新建轨道_0)))
        (:Backward
          (Class|PlayerController|AddPitchInput _returnvalue (* (Math|Float|Lerp 0.0 -0.15 _新建轨道_0) -1.0)))))
    (:Finished
      (CallFunction|重置后座力Event)
      (Utilities|FlowControl|RetriggerableDelay 0.05)
      (CallFunction|停止晃动Event))))

(event Custom|松开“fire”
  ;[1 1 1] 武器开火
  (Default|武器开火（由人物调用） (Variables|Default|GetWeaponComponent) false))

(event Custom|LoadAmmo
  ;[1 1 1] 重装子弹
  (Default|重装弹药 (Variables|Default|GetWeaponComponent)))

(event Custom|重置后座力Event
  (bind _returnvalue (Game|GetPlayerController 0))
  ;[1 1 1] 后座力
  (bind (_direction _新建轨道_0) (Timeline|时间轴_1 Reverse)
    (:Update
      (switch Utilities|FlowControl|Switch|SwitchonETimelineDirection _direction
        (:Forward
          (Class|PlayerController|AddPitchInput _returnvalue (Math|Float|Lerp 0.0 -0.15 _新建轨道_0)))
        (:Backward
          (Class|PlayerController|AddPitchInput _returnvalue (* (Math|Float|Lerp 0.0 -0.15 _新建轨道_0) -1.0)))))
    (:Finished
      (CallFunction|重置后座力Event)
      (Utilities|FlowControl|RetriggerableDelay 0.05)
      (CallFunction|停止晃动Event))))

(event Custom|停止晃动Event
  (bind _returnvalue (Game|GetPlayerController 0))
  ;[1 1 1] 后座力
  (bind (_direction _新建轨道_0) (Timeline|时间轴_1 Stop)
    (:Update
      (switch Utilities|FlowControl|Switch|SwitchonETimelineDirection _direction
        (:Forward
          (Class|PlayerController|AddPitchInput _returnvalue (Math|Float|Lerp 0.0 -0.15 _新建轨道_0)))
        (:Backward
          (Class|PlayerController|AddPitchInput _returnvalue (* (Math|Float|Lerp 0.0 -0.15 _新建轨道_0) -1.0)))))
    (:Finished
      (CallFunction|重置后座力Event)
      (Utilities|FlowControl|RetriggerableDelay 0.05)
      (CallFunction|停止晃动Event))))

(event Custom|Equip/Unequip
  ;[1 1 1] 装备武器
  (Default|装备武器（收枪与拔枪的逻辑） (Variables|Default|GetWeaponComponent)))

(event Custom|EquipWeapon
  (bind _currweapon (Variables|Default|GetCurrWeapon))
  (bind _weapon_info (Variables|/Game/Game_Files/Weapon/BaseWeapon_BP.BaseWeapon_BP_C|GetWeapon_info _currweapon))
  (bind (_武器伤害值 _weaponholdsocket _weaponequipsocket _unequipsound _equipsound) (Utilities|Struct|Breakweapon_Info _weapon_info))
  ;[1 1 1] 装备武器
  (Transformation|AttachComponentToComponent _currweapon (Variables|Character|GetMesh) _weaponequipsocket "SnapToTarget" "SnapToTarget" "SnapToTarget" true)
  (Audio|PlaySound2D _equipsound 1.0 1.0 0.0 0 0))

(event Custom|拾取武器
  (params (Weapon_Ref :type Weapon%20BP%20Child%20Object%20Reference))
  ;[1 1 1] 捡取武器
  (Default|挂载或装备武器 (Variables|Default|GetWeaponComponent) Weapon_Ref)
  (Variables|Default|SetOverlapWeapon_New 0))

(event Custom|UnequipWeapon
  (bind _currweapon (Variables|Default|GetCurrWeapon))
  (bind _weapon_info (Variables|/Game/Game_Files/Weapon/BaseWeapon_BP.BaseWeapon_BP_C|GetWeapon_info _currweapon))
  (bind (_武器伤害值 _weaponholdsocket _weaponequipsocket _unequipsound _equipsound) (Utilities|Struct|Breakweapon_Info _weapon_info))
  ;[1 1 1] 装备武器
  (Transformation|AttachComponentToComponent _currweapon (Variables|Character|GetMesh) _weaponholdsocket "SnapToTarget" "SnapToTarget" "SnapToTarget" true)
  (Audio|PlaySound2D _unequipsound 1.0 1.0 0.0 0 0))

(event Custom|SwitchWeapon
  ;[1 1 1] 按顺序快速切换枪支
  (Default|顺序切换武器 (Variables|Default|GetWeaponComponent)))

(event Custom|Unequip
  ;[1 1 1] 装备武器
  (Variables|Default|SetHandWithWeapon false)
  (bind _returnvalue (Animation|PlayAnimMontage "/Game/AnimStarterPack/UnEquip_Rifle_Standing_Montage1.UnEquip_Rifle_Standing_Montage1" 2.5 "None"))
  (Variables|Default|SetHoldTime _returnvalue)
  (CallFunction|行动模式 false true))

(event Custom|Equip
  ;[1 1 1] 装备武器
  (Variables|Default|SetHandWithWeapon true)
  (Animation|PlayAnimMontage "/Game/AnimStarterPack/Equip_Rifle_Standing_Montage.Equip_Rifle_Standing_Montage" 2.5 "None")
  (CallFunction|行动模式 true false))

(event Custom|根据需求切换武器
  (params (待切换的武器名字 :type Text))
  ;[1 1 1] 根据需求切换武器
  (Default|一键切换武器 (Variables|Default|GetWeaponComponent) 待切换的武器名字))

(event EventTransimitDamage
  (params (Damage :type Float%20%28single-precision%29))
  ;[1 1 1] 人物受到伤害
  (bind _output_get (Variables|Default|SetCurrentHealth (- (Variables|Default|GetCurrentHealth) Damage)))
  (bind _output_get_2 (Variables|Default|SetPlayerDead? (<= _output_get 0.0)))
  (if _output_get_2
    (Input|DisableInput (Game|GetPlayerController 0))
    (else
      (Animation|PlayAnimMontage "/Game/AnimStarterPack/Hit_React_2_Montage.Hit_React_2_Montage" 1.0 "None"))))

(event Input|AxisEvents|InputAxisMoveForward
  (params (AxisValue :type Float%20%28single-precision%29))
  (bind _returnvalue (Pawn|GetControlRotation :!class /Script/Engine.Pawn))
  (bind _weaponcomponent (Variables|Default|GetWeaponComponent))
  (bind _returnvalue_2 (Math|Vector|GetForwardVector _returnvalue))
  (bind _weaponinhand_ (Variables|/Game/Game_Files/WeaponComponent/WeaponComponent.WeaponComponent_C|GetWeaponInHand? _weaponcomponent))
  ;[1 1 1] 移动
  (Math|Float|CompareFloat AxisValue 1.0
    (:>
      (Pawn|Input|AddMovementInput _returnvalue_2 AxisValue false :!label _label)
      (if _weaponinhand_
        (CallFunction|行动模式 false true)
        (bind _新建轨道_0 (Timeline|时间轴_0 Play)
          (:Update
            (Variables|/Script/Engine.CharacterMovementComponent|SetMaxWalkSpeed (Variables|Character|GetCharacterMovement) (Math|Float|Lerp 3e+02 6e+02 _新建轨道_0))))))
    (:==
      (goto _label))
    (:<
      (Pawn|Input|AddMovementInput _returnvalue_2 AxisValue false)
      (if _weaponinhand_
        (CallFunction|行动模式 true false)
        (Timeline|时间轴_0 Reverse)))))

(event Input|AxisEvents|InputAxisMoveRight
  (params (AxisValue :type Float%20%28single-precision%29))
  ;[1 1 1] 移动
  (Pawn|Input|AddMovementInput (Math|Vector|GetRightVector (Pawn|GetControlRotation :!class /Script/Engine.Pawn)) AxisValue false))

(event Input|AxisEvents|InputAxisTurn
  (params (AxisValue :type Float%20%28single-precision%29))
  ;[1 1 1] 左右转
  (Pawn|Input|AddControllerYawInput AxisValue))

(event Input|AxisEvents|InputAxisLookUp
  (params (AxisValue :type Float%20%28single-precision%29))
  ;[1 1 1] 左右转
  (Pawn|Input|AddControllerPitchInput AxisValue))

(event Custom|input%20touch
  (Utilities|FlowControl|Gate true
    (:Exit
      (if (>= (Math|Vector2D|Vector2DLength (- (Math|Vector2D|MakeVector2D (.LocationX (Class|PlayerController|GetInputTouchState (Game|GetPlayerController 0) (stale Input|TouchEvents|InputTouch FingerIndex))) (.LocationY (Class|PlayerController|GetInputTouchState (Game|GetPlayerController 0) (stale Input|TouchEvents|InputTouch FingerIndex)))) (Variables|Default|Get下一触控位置))) (Variables|Default|Get旋转的速率))
        (Variables|Default|Set触控位置 (Variables|Default|Get下一触控位置))
        (Pawn|Input|AddControllerYawInput (.x (* (- (Math|Vector2D|MakeVector2D (.LocationX (Class|PlayerController|GetInputTouchState (Game|GetPlayerController 0) (stale Input|TouchEvents|InputTouch FingerIndex))) (.LocationY (Class|PlayerController|GetInputTouchState (Game|GetPlayerController 0) (stale Input|TouchEvents|InputTouch FingerIndex)))) (Variables|Default|Get下一触控位置)) (Variables|Default|Get旋转的速率))))
        (Pawn|Input|AddControllerPitchInput (.y (* (- (Math|Vector2D|MakeVector2D (.LocationX (Class|PlayerController|GetInputTouchState (Game|GetPlayerController 0) (stale Input|TouchEvents|InputTouch FingerIndex))) (.LocationY (Class|PlayerController|GetInputTouchState (Game|GetPlayerController 0) (stale Input|TouchEvents|InputTouch FingerIndex)))) (Variables|Default|Get下一触控位置)) (Variables|Default|Get旋转的速率))))))))

(event Input|TouchEvents|InputTouch
  (params (Location :type Vector) (FingerIndex :type ETouchIndex%20Enum))
  (bind _returnvalue (Game|GetPlayerController 0))
  (bind (_locationx _locationy) (Class|PlayerController|GetInputTouchState _returnvalue FingerIndex))
  (bind _returnvalue_2 (Math|Vector2D|MakeVector2D _locationx _locationy))
  (:Pressed
    (bind _output_get (Variables|Default|Set触控位置 _returnvalue_2))
    (Variables|Default|Set下一触控位置 _output_get)
    (Utilities|FlowControl|Gate true) ; enters at Open
  )
  (:Released
    (Utilities|FlowControl|Gate true) ; enters at Close
  ))

(fn ConstructionScript)

(fn 行动模式
  (params (使用控制器旋转Yaw :type Boolean) (将旋转朝向运动 :type Boolean))
  (Variables|Default|SetbUseControllerRotationYaw 使用控制器旋转Yaw)
  (Variables|/Script/Engine.CharacterMovementComponent|SetbOrientRotationToMovement (Variables|Character|GetCharacterMovement) 将旋转朝向运动))
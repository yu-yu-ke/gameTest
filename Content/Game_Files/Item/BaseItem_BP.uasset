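; BaseItem_BP is a base item actor that builds its visual mesh from the item ID (物品ID) in its PackageItemInfo.
; The Construction Script looks up the item's mesh type, then dynamically adds either a static or skeletal mesh component with the matching asset.
; The new component is stored in ItemStaticMesh or ItemSketecalMesh.
; The Event Graph holds only disabled placeholder events, so the Blueprint has no runtime logic of its own.
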(event EventBeginPlay)

(event Collision|EventActorBeginOverlap
  (params (OtherActor :type Actor%20Object%20Reference)))

(event EventTick
  (params (DeltaSeconds :type Float%20%28single-precision%29)))

(fn ConstructionScript
  (bind _packageitem_info (Variables|Default|GetPackageItem_Info))
  (bind _物品id (Utilities|Struct|BreakPackageSlot_Info _packageitem_info))
  (switch Utilities|FlowControl|Switch|SwitchonMeshType (CallFunction|获得物品Mesh类型 _物品id)
    (:NewEnumerator0
      (bind _returnvalue (AddComponent|AddStaticMeshComponent false))
      (Components|StaticMesh|SetStaticMesh _returnvalue (CallFunction|获得物品静态网格体 _物品id))
      (Variables|Default|SetItemStaticMesh _returnvalue))
    (:NewEnumerator1
      (bind _returnvalue_2 (AddComponent|AddSkeletalMeshComponent false))
      (Class|SkinnedMeshComponent|SetSkeletalMesh _returnvalue_2 (CallFunction|获得物品骨骼网格体 _物品id) true)
      (Variables|Default|SetItemSketecalMesh _returnvalue_2))))
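; Ammo_BP is a projectile actor for the weapon system, configured by its AmmoInfo struct.
; The construction script builds the mesh and trail and sets projectile speeds.
; When the projectile stops, it sends direct damage through Transimit_Damage_Interface, or radius damage via sphere overlap plus a spawned Boom actor.
; It then hides its mesh, spawns the impact effect from player 0's current weapon, and expires shortly after.
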(event OnProjectileStop(ProjectileMovement)
  (params (ImpactResult :type Hit%20Result%20Structure%20%28by%20ref%29))
  (CallFunction|发射物撞击停止函数 self ImpactResult))

(fn ConstructionScript
  (bind _projectilemovement (Variables|Default|GetProjectileMovement))
  (Utilities|FlowControl|Sequence
    (:then_0
      (bind _returnvalue (AddComponent|AddStaticMeshComponent false))
      (Components|StaticMesh|SetStaticMesh _returnvalue (.子弹模型 (Utilities|Struct|BreakAmmo_Info (Variables|Default|GetAmmo_Info))))
      (Variables|Default|Set弹药模型 _returnvalue)
      (Variables|/Script/Engine.ProjectileMovementComponent|SetInitialSpeed _projectilemovement (.子弹发射的初始速度 (Utilities|Struct|BreakAmmo_Info (Variables|Default|GetAmmo_Info)))))
    (:then_1
      (bind _returnvalue_2 (AddComponent|AddParticleSystemComponent false))
      (Effects|Components|ParticleSystem|SetTemplate _returnvalue_2 (.子弹拖尾效果 (Utilities|Struct|BreakAmmo_Info (Variables|Default|GetAmmo_Info))))
      (Variables|Default|Set拖尾效果 _returnvalue_2)
      (Variables|/Script/Engine.ProjectileMovementComponent|SetMaxSpeed _projectilemovement (.子弹发射后的最大速度 (Utilities|Struct|BreakAmmo_Info (Variables|Default|GetAmmo_Info))))))
  (Variables|Default|SetAmmo_Info (Utilities|Struct|MakeAmmo_Info (.子弹类型 (Variables|Default|GetAmmo_Info)) (.子弹模型 (Variables|Default|GetAmmo_Info)) (.子弹直接命中的伤害值 (Variables|Default|GetAmmo_Info)) (.子弹发射的初始速度 (Variables|Default|GetAmmo_Info)) (.子弹发射后的最大速度 (Variables|Default|GetAmmo_Info)) (Utilities|GetClass self) (.子弹拖尾效果 (Variables|Default|GetAmmo_Info)) (.是否具有径向爆炸伤害 (Variables|Default|GetAmmo_Info)) (.径向爆炸伤害值 (Variables|Default|GetAmmo_Info)) (.爆炸半径 (Variables|Default|GetAmmo_Info)) (.爆炸强度 (Variables|Default|GetAmmo_Info)))))

(fn 发射物撞击停止函数
  (params (命中结果 :type Hit%20Result%20Structure))
  (bind _returnvalue (Game|Player|GetPlayerPawn 0))
  (bind _returnvalue_2 (Actor|GetComponentbyClass _returnvalue "/Game/Game_Files/WeaponComponent/WeaponComponent.WeaponComponent_C"))
  (bind _currentweapon (Variables|/Game/Game_Files/WeaponComponent/WeaponComponent.WeaponComponent_C|GetCurrentWeapon _returnvalue_2))
  (bind _weapon_info (Variables|/Game/Game_Files/Item/Weapon_Child/Weapon_BP_Child.Weapon_BP_Child_C|GetWeapon_Info _currentweapon))
  (bind _特效信息 (Utilities|Struct|BreakWeapon_Info _weapon_info))
  (LocalVariables|SetTemp_HitResult 命中结果)
  (Utilities|FlowControl|Sequence
    (:then_0
      (if (Utilities|Struct|BreakAmmo_Info (Variables|Default|GetAmmo_Info))
        (CallFunction|径向爆炸函数 (LocalVariables|GetTemp_HitResult))
        (elif (Utilities|DoesObjectImplementInterface (.HitActor (Collision|BreakHitResult (LocalVariables|GetTemp_HitResult))) "/Game/Game_Files/BP_Interface/Transimit_Damage_Interface.Transimit_Damage_Interface_C")
          (Class|TransimitDamageInterface|TransimitDamage(Message) (.HitActor (Collision|BreakHitResult (LocalVariables|GetTemp_HitResult))) (LocalVariables|GetTemp_HitResult) (Utilities|Struct|BreakAmmo_Info (Variables|Default|GetAmmo_Info))))))
    (:then_1
      (Development|SetHiddeninGame (Variables|Default|Get弹药模型) true false)
      (Game|SpawnActorfromClass (Utilities|Struct|BreakEffect_Info _特效信息) (Math|Transform|MakeTransform "0, 0, 0" "0, 0, 0" "1,1,1") "Undefined" 0 _特效信息 (LocalVariables|GetTemp_HitResult) 0)
      (Actor|SetLifeSpan 0.1))))

(fn 径向爆炸函数
  (params (命中结果 :type Hit%20Result%20Structure))
  (bind _ammo_info (Variables|Default|GetAmmo_Info))
  (bind (_爆炸半径 _爆炸强度) (Utilities|Struct|BreakAmmo_Info _ammo_info))
  (LocalVariables|SetTemp_HitResult 命中结果)
  (Utilities|FlowControl|Sequence
    (:then_0
      (bind _outactors (Collision|SphereOverlapActors (.ImpactPoint (Collision|BreakHitResult (LocalVariables|GetTemp_HitResult))) (Utilities|Struct|BreakAmmo_Info (Variables|Default|GetAmmo_Info)) (Utilities|Array|MakeArray "ObjectTypeQuery1" "ObjectTypeQuery2" "ObjectTypeQuery3" "ObjectTypeQuery6" "ObjectTypeQuery5" "ObjectTypeQuery4") 0 (Utilities|Array|MakeArray (Variables|/Game/Game_Files/WeaponComponent/WeaponComponent.WeaponComponent_C|GetCurrentWeapon (Actor|GetComponentbyClass (Game|Player|GetPlayerPawn 0) "/Game/Game_Files/WeaponComponent/WeaponComponent.WeaponComponent_C")))))
      (for _array_element _outactors
        (if (Utilities|DoesObjectImplementInterface _array_element "/Game/Game_Files/BP_Interface/Transimit_Damage_Interface.Transimit_Damage_Interface_C")
          (Class|TransimitDamageInterface|TransimitRadiusDamage(Message) _array_element (LocalVariables|GetTemp_HitResult) (Variables|Default|GetAmmo_Info)))))
    (:then_1
      (Game|SpawnActorfromClass "/Game/Game_Files/WeaponComponent/Ammo/Boom.Boom_C" (Math|Transform|MakeTransform (.ImpactPoint (Collision|BreakHitResult (LocalVariables|GetTemp_HitResult))) "0, 0, 0" "1,1,1") "Undefined" 0 _爆炸强度 _爆炸半径 0))))